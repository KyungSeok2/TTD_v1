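; Enemy spawner actor that releases AI monsters in repeating timed attack waves.
; A looping timer started at BeginPlay triggers each attack, which runs a looping spawn timer at SpawnCoolTime until a shorter one-shot timer clears it.
; Each spawn creates an AI_Monster running BT_TTD_Monster_AI at one of three random spawn points, always using SpawnPoint1's rotation.
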(event EventBeginPlay
  (Variables|Default|SetSpawnPointArray (Utilities|Array|MakeArray (Variables|Default|GetSpawnPoint2) (Variables|Default|GetSpawnPoint3) (Variables|Default|GetSpawnPoint1)))
  (Utilities|Time|SetTimerbyFunctionName 0 "Start Attack" 25.0 true))

(fn ConstructionScript)

(fn SpawnEnemy
  (AI|SpawnAIFromClass "/Game/a_TTD/Blueprints/AI_Monster.AI_Monster_C" "/Game/a_TTD/Blueprints/AI_BP/BT_TTD_Monster_AI.BT_TTD_Monster_AI" (Transformation|GetWorldLocation (.OutItem (Utilities|Array|Random (Variables|Default|GetSpawnPointArray)))) (Transformation|GetWorldRotation (Variables|Default|GetSpawnPoint1)) false 0))

(fn StopSpawnEnemy
  (Utilities|Time|ClearTimerbyFunctionName 0 "Spawn Enemy"))

(fn SpawnEnemyDu
  (Utilities|Time|SetTimerbyFunctionName 0 "Spawn Enemy" (Variables|Default|GetSpawnCoolTime) true))

(fn StartAttack
  (CallFunction|SpawnEnemyDu)
  (Utilities|Time|SetTimerbyFunctionName 0 "Stop Spawn Enemy" 15.0))