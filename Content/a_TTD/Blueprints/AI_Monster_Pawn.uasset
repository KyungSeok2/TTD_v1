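; AI monster pawn with an AI Perception component, apparently meant to target player towers through a Blackboard key.
; Both perception events are empty, and the nearest-tower search over actors tagged PlayerTower is disconnected debug-laden logic that never runs.
; CheckTowerActor clears the tower key if it holds a valid object, otherwise stores the sensed actor, but nothing in this Blueprint calls it.
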(event OnPerceptionUpdated(AIPerception)
  (params (UpdatedActors :type Array%20of%20Actor%20Object%20References)))

(event OnTargetPerceptionUpdated(AIPerception)
  (params (Actor :type Actor%20Object%20Reference) (Stimulus :type AI%20Stimulus%20Structure)))

(fn ConstructionScript)

(fn CheckTowerActor
  (params (SensedActor :type Actor%20Object%20Reference))
  (Utilities|IsValid (AI|Components|Blackboard|GetValueasObject (AI|GetBlackboard 0) (Variables|Default|GetPlayerTowerKey))
    (:Is%20Valid
      (AI|Components|Blackboard|SetValueasObject (AI|GetBlackboard 0) (Variables|Default|GetPlayerTowerKey) 0))
    (:Is%20Not%20Valid
      (AI|Components|Blackboard|SetValueasObject (AI|GetBlackboard 0) (Variables|Default|GetPlayerTowerKey) SensedActor))))