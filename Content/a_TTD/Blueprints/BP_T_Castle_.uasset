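; Castle tower actor for the tabletop defense game that takes damage and slowly self-repairs.
; On BeginPlay it registers with the TableTopDefense game mode and starts a looping timer that restores HP up to a cap.
; Damage reduces HP; at zero it spawns a large explosion, destroys itself after a short delay, then calls SetTowers on the game mode.
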(event EventBeginPlay
  (bind _asbp_gm_table_top_defense (Utilities|Casting|CastToBP_GM_TableTopDefense (Game|GetGameMode)))
  (Default|AddTower _asbp_gm_table_top_defense self)
  (Utilities|Time|SetTimerbyFunctionName 0 "Repair" 5.0 true))

(event Game|Damage|EventAnyDamage
  (params (Damage :type Float%20%28single-precision%29) (DamageType :type Damage%20Type%20Object%20Reference) (InstigatedBy :type Controller%20Object%20Reference) (DamageCauser :type Actor%20Object%20Reference))
  (bind _output_get (Variables|Default|SetHP (- (Variables|Default|GetHP) Damage)))
  (if (<= _output_get 0.0)
    (Effects|SpawnEmitteratLocation "/Game/StarterContent/Particles/P_Explosion.P_Explosion" (Transformation|GetWorldLocation (Variables|Default|GetStaticMesh)) "0, 0, 0" "20.000000,20.000000,20.000000")
    (Utilities|FlowControl|Delay 0.5)
    (Actor|DestroyActor)
    (bind _asbp_gm_table_top_defense (Utilities|Casting|CastToBP_GM_TableTopDefense (Game|GetGameMode)))
    (Default|SetTowers _asbp_gm_table_top_defense)))

(fn ConstructionScript)

(fn Repair
  (Variables|Default|SetHP (Math|Float|Clamp(Float) (+ (Variables|Default|GetHP) 7.0) 0.0 1e+04)))