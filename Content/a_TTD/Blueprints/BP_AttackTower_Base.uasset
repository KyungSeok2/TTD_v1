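; Base attack tower that fires arrows at enemies, apparently for a tower defense game.
; If Build is set at BeginPlay, it enables mesh collision and starts a looping cooldown timer calling Find Nearest Enemy.
; That function sphere-traces upward from ShootPoint at AttackRange radius and, if the single hit is tagged Enemy, spawns AI_Pawn_Arrow aimed at it.
; Despite its name, it compares no distances; debug drawing and disconnected damage nodes remain.
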(event EventBeginPlay
  (|CallParentFunction)
  (if (Variables|Default|GetBuild??)
    (Collision|SetCollisionEnabled (Variables|Default|GetStaticMesh) "QueryAndPhysics")
    (Utilities|Time|SetTimerbyFunctionName 0 "Find Nearest Enemy" (Variables|Default|GetAttackCoolTime) true)))

(fn ConstructionScript
  (|CallParentFunction))

(fn Build
  (Variables|Default|SetBuild?? true))

(fn FindNearestEnemy
  (bind _shootpoint (Variables|Default|GetShootPoint))
  (bind _returnvalue (Transformation|GetWorldLocation _shootpoint))
  (bind (_x _y _z) (Math|Vector|BreakVector _returnvalue))
  (bind (_outhit _returnvalue_2) (Collision|SphereTraceByChannel _returnvalue (Math|Vector|MakeVector _x _y (+ _z 2e+03)) (Variables|Default|GetAttackRange) "TraceTypeQuery4" false 0 "ForDuration"))
  (if _returnvalue_2
    (if (Actor|ActorHasTag (.HitActor (Collision|BreakHitResult _outhit)) "Enemy")
      (bind _output_get (Variables|Default|SetTargetEnemy (.HitActor (Collision|BreakHitResult _outhit))))
      (Game|SpawnActorfromClass "/Game/a_TTD/Blueprints/AI_Pawn_Arrow.AI_Pawn_Arrow_C" (Math|Transform|MakeTransform (Transformation|GetWorldLocation (Variables|Default|GetShootPoint1)) (Math|Rotator|FindLookatRotation (Transformation|GetWorldLocation (Variables|Default|GetShootPoint1)) (Transformation|GetActorLocation _output_get)) "1,1,1") "Undefined" 0 0)
      (else
        (Development|PrintString "Hello")))))