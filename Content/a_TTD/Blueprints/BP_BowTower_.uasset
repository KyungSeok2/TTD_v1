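; BP_BowTower is a bow tower Blueprint that extends a parent tower class with its own build and upgrade behavior.
; SetBuild runs the parent logic, then sets a fixed world rotation on the SML3 component.
; Upgrade calls the parent, then reads the game mode's UpgradeLevel to change visuals by mesh swap or by revealing SML3.
; Each level also raises HP and sets max HP, attack cooldown, range and damage.
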(event EventBeginPlay
  (|CallParentFunction) ; 지금 이 노드는 비활성 상태입니다. \n핀을 끌어서 다른 노드를 연결하면 활성화됩니다.
)

(event Collision|EventActorBeginOverlap
  (params (OtherActor :type Actor%20Object%20Reference)))

(event EventTick
  (params (DeltaSeconds :type Float%20%28single-precision%29)))

(fn ConstructionScript
  (|CallParentFunction))

(fn SetBuild
  (Utilities|FlowControl|Sequence
    (:then_0
      (|CallParentFunction))
    (:then_1
      (Transformation|SetWorldRotation (Variables|Default|GetSM_L3) "0,24.000000, 0" false false))))

(fn Upgrade
  (|CallParentFunction)
  (switch Utilities|FlowControl|Switch|SwitchonBP_UpgradeLevel (Variables|/Game/a_TTD/GameMode/BP_GM_TableTopDefense.BP_GM_TableTopDefense_C|GetUpgrade%20Level%20 (Variables|Default|GetTTD_GameMode))
    (:NewEnumerator1
      (Components|StaticMesh|SetStaticMesh (Variables|Default|GetStaticMesh) 0)
      (Variables|Default|SetMaxHP 5e+03)
      (Variables|Default|SetHP (+ (Variables|Default|GetHP) (Variables|Default|GetMaxHP)))
      (Variables|Default|SetAttackCoolTime 0.4)
      (Variables|Default|SetAttackRange 4e+03)
      (Variables|Default|SetDamage 75.0))
    (:NewEnumerator2
      (Rendering|SetVisibility (Variables|Default|GetSM_L3) true false)
      (Variables|Default|SetMaxHP 7e+03)
      (Variables|Default|SetHP (+ (Variables|Default|GetHP) (Variables|Default|GetMaxHP)))
      (Variables|Default|SetAttackCoolTime 0.3)
      (Variables|Default|SetAttackRange 5e+03)
      (Variables|Default|SetDamage 1e+02))))