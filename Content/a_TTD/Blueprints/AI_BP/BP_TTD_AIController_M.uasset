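; AI controller for monsters in the tabletop defense game, pointing them at player towers.
; On BeginPlay it runs the monster behavior tree, calls FindTower after a short delay, and binds to the game mode's tower-update dispatcher.
; FindTower copies valid towers from the game mode, then writes the nearest one and a random reachable point around it to the Blackboard.
; ClearTowerKey empties the tower target key.
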(event EventBeginPlay
  (Utilities|FlowControl|Sequence
    (:then_0
      (AI|RunBehaviorTree "/Game/a_TTD/Blueprints/AI_BP/BT_TTD_Monster_AI.BT_TTD_Monster_AI")
      (Utilities|FlowControl|Delay 0.2)
      (CallFunction|FindTower))
    (:then_1
      (bind _asbp_gm_table_top_defense (Utilities|Casting|CastToBP_GM_TableTopDefense (Game|GetGameMode))
        (:then
          (EventDispatchers|BindEventtoEventDispatcherUpdateTower _asbp_gm_table_top_defense (EventDispatchers|CreateEvent :!event ClearTowerKey)))
        (:CastFailed
          (Development|PrintString "AIC _GM Cast Fail"))))))

(fn ConstructionScript)

(fn FindTower
  (bind _self self)
  (bind _blackboard (Variables|Default|GetBlackboard))
  (bind _updated_towers_ac (Variables|Default|GetUpdated%20Towers%20AC))
  (bind _returnvalue (Pawn|GetControlledPawn _self))
  (bind _returnvalue_2 (Transformation|GetActorLocation _returnvalue))
  (bind _returnvalue_3 (Actor|FindNearestActor _returnvalue_2 _updated_towers_ac))
  (Utilities|Array|Clear (Variables|Default|GetUpdated%20Towers%20AC))
  ;[1 1 1] 블랙보드의 값 비우기
  (AI|Components|Blackboard|SetValueasObject (Variables|Default|GetBlackboard) (Utilities|Name|MakeLiteralName "PlayerTowerKey") 0)
  ;[1 1 1] 게임모드에서 설치된 타워 배열 가져오기
  (bind _asbp_gm_table_top_defense (Utilities|Casting|CastToBP_GM_TableTopDefense (Game|GetGameMode)))
  (for _array_element (Variables|/Game/a_TTD/GameMode/BP_GM_TableTopDefense.BP_GM_TableTopDefense_C|GetUpdateTowers _asbp_gm_table_top_defense)
    (Utilities|IsValid _array_element
      (:Is%20Valid
        ;[1 1 1] 배열에 넣기
        (Utilities|Array|Add (Variables|Default|GetUpdated%20Towers%20AC) _array_element))))
  ;[1 1 1] 첫번째 배열에 값이 있는지 확인
  (if (Utilities|Array|IsValidIndex (Variables|Default|GetUpdated%20Towers%20AC))
    ;[1 1 1] 블랙보드에 값 입력
    (AI|Components|Blackboard|SetValueasObject _blackboard (Utilities|Name|MakeLiteralName "PlayerTowerKey") _returnvalue_3)
    (AI|Components|Blackboard|SetValueasVector _blackboard (Utilities|Name|MakeLiteralName "PlayerTowerLocationKey") (.RandomLocation (AI|Navigation|GetRandomReachablePointinRadius (Transformation|GetActorLocation _returnvalue_3) 4e+02 0 0)))))

(fn ClearTowerKey
  (AI|Components|Blackboard|SetValueasObject (Variables|Default|GetBlackboard) (Utilities|Name|MakeLiteralName "PlayerTowerKey") 0))