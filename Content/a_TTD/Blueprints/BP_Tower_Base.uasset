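; Base tower actor for a tabletop tower defense game with motion-controller grabbing, providing placement, health and destruction.
; A timer-driven downward trace moves a preview marker over Landscape, turning it red on invalid spots.
; Building snaps the tower to the traced point, disables physics, plays haptics and registers with the game mode.
; It self-repairs periodically, explodes at zero HP, and leaves Upgrade as an empty hook bound to the game mode's dispatcher.
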(event EventBeginPlay
  (bind _asbp_gm_table_top_defense (Utilities|Casting|CastToBP_GM_TableTopDefense (Game|GetGameMode)))
  (bind _output_get (Variables|Default|SetTTD_GameMode _asbp_gm_table_top_defense))
  (EventDispatchers|BindEventtoEventDispatcherUpgrade _output_get (EventDispatchers|CreateEvent :!event Upgrade))
  (CallFunction|Upgrade)
  (Utilities|Time|SetTimerbyFunctionName 0 "Repair" 3.0 true)
  (if (Variables|Default|GetBuild?)
    (build|BuildTower)))

(event Game|Damage|EventAnyDamage
  (params (Damage :type Float%20%28single-precision%29) (DamageType :type Damage%20Type%20Object%20Reference) (InstigatedBy :type Controller%20Object%20Reference) (DamageCauser :type Actor%20Object%20Reference))
  (attack|AddDamage Damage))

(fn ConstructionScript)

(fn FindBuildLocation
  (bind _buildpoint (Variables|Default|GetBuildPoint))
  (bind (_hit_location _hit_linetrace _hit_landscape) (attack|LintraceforDown))
  (if _hit_linetrace
    (if (and _hit_landscape (not (Class|PrimitiveComponent|IsOverlappingComponent (Variables|Default|GetBuildPoint))))
      (Transformation|SetWorldLocation (Variables|Default|GetBuildPoint) _hit_location false false)
      (Rendering|Material|SetMaterial _buildpoint 0 "/Game/EF_FirstFloor/Common/Materials/Glass/WM_GlassClean_a.WM_GlassClean_a")
      (Rendering|SetVisibility _buildpoint true false)
      (else
        (Rendering|Material|SetMaterial _buildpoint 0 "/Game/a_TTD/Material/M_Red.M_Red")))
    (else
      (Rendering|SetVisibility _buildpoint false false))))

(fn FindBuildLocationDu
  (Utilities|Time|SetTimerbyFunctionName 0 "Find Build Location" 0.1 true))

(fn LintraceforDown
  (bind _cylinder (Variables|Default|GetCylinder))
  (bind _returnvalue (Transformation|GetWorldLocation _cylinder))
  (bind (_x _y _z) (Math|Vector|BreakVector _returnvalue))
  (bind (_outhit _returnvalue_2) (Collision|LineTraceForObjects _returnvalue (Math|Vector|MakeVector _x _y (- _z 3e+03)) (Utilities|Array|MakeArray "ObjectTypeQuery2" "ObjectTypeQuery1" "ObjectTypeQuery9") false 0 "None"))
  (return (.Location (Collision|BreakHitResult _outhit)) _returnvalue_2 (== (Utilities|GetClass (.HitActor (Collision|BreakHitResult _outhit))) "/Script/Landscape.Landscape")))

(fn BuildTower
  (bind (_hit_location _hit_linetrace _hit_landscape) (attack|LintraceforDown))
  (if _hit_linetrace
    (if _hit_landscape
      (Transformation|SetActorLocationAndRotation _hit_location (Math|Rotator|MakeRotator 0.0 0.0 (.yaw (Transformation|GetActorRotation))))
      (Physics|SetSimulatePhysics (Variables|Default|GetStaticMesh) false)
      (build|SetBuild)
      (Variables|Default|SetBuild? true)
      (Default|AddTower (Variables|Default|GetTTD_GameMode) self))))

(fn StopFindBuildLocation
  (Utilities|Time|ClearTimerbyFunctionName 0 "Find Build Location"))

(fn SetBuild
  ;[1 1 1] 건설될때 자식 엑터가 장동시킬 함수
  (Rendering|SetVisibility (Variables|Default|GetBuildPoint) false false)
  (Class|MagicLeapControllerFunctionLibrary|PlayHapticPattern (Variables|/Script/HeadMountedDisplay.MotionControllerComponent|GetMotionSource (Variables|/Game/VRTemplate/Blueprints/GrabComponent.GrabComponent_C|GetMotionControllerRef (Variables|Default|GetGrabComponent))) "Bump" "High"))

(fn Upgrade)

(fn Repair
  (Variables|Default|SetHP (Math|Float|Clamp(Float) (+ (Variables|Default|GetHP) (Variables|Default|Getrepair_HP)) 0.0 (Variables|Default|GetMaxHP))))

(fn AddDamage
  (params (Damage :type Float%20%28single-precision%29))
  (bind _output_get (Variables|Default|SetHP (- (Variables|Default|GetHP) Damage)))
  (if (<= _output_get 0.0)
    (Audio|PlaySoundatLocation "/Game/StarterContent/Audio/Explosion_Cue.Explosion_Cue" "0, 0, 0" "0, 0, 0" 1.0 1.0 0.0 0 0 0)
    (Effects|SpawnEmitteratLocation "/Game/StarterContent/Particles/P_Explosion.P_Explosion" (Transformation|GetWorldLocation (Variables|Default|GetStaticMesh)) "0, 0, 0" "20.000000,20.000000,20.000000")
    (Actor|DestroyActor)
    (Default|SetTowers (Variables|Default|GetTTD_GameMode))))