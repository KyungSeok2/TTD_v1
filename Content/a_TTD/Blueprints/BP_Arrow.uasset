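; BP_Arrow is a homing projectile that damages enemies on impact.
; Shoot turns on homing in its ProjectileMovement toward a target component with a very high acceleration, so the arrow tracks its target tightly.
; A setter stores the damage, which the static mesh's hit event applies to actors tagged Enemy before destroying the arrow.
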(event OnComponentHit(StaticMesh)
  (params (HitComponent :type Primitive%20Component%20Object%20Reference) (OtherActor :type Actor%20Object%20Reference) (OtherComp :type Primitive%20Component%20Object%20Reference) (NormalImpulse :type Vector :default "0, 0, 0") (Hit :type Hit%20Result%20Structure%20%28by%20ref%29))
  (if (Actor|ActorHasTag OtherActor "Enemy")
    (Game|Damage|ApplyDamage OtherActor (Variables|Default|GetDamage) 0 0)
    (Actor|DestroyActor)))

(fn ConstructionScript)

(fn Shoot
  (params (Target :type Scene%20Component%20Object%20Reference))
  (bind _projectilemovement (Variables|Default|GetProjectileMovement))
  (Variables|/Script/Engine.ProjectileMovementComponent|SetbIsHomingProjectile _projectilemovement true)
  (Variables|/Script/Engine.ProjectileMovementComponent|SetHomingAccelerationMagnitude _projectilemovement 99999.0)
  (Variables|/Script/Engine.ProjectileMovementComponent|SetHomingTargetComponent _projectilemovement Target))

(fn SetDamageArrow
  (params (Damage :type Float%20%28single-precision%29))
  (Variables|Default|SetDamage Damage))