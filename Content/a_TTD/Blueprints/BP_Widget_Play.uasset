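; BP_Widget_Play is a Blueprint that keeps its Widget component turned toward the player's camera, acting as a world-space billboard.
; BeginPlay casts player pawn 0 to BP_TTD_Character and caches the reference.
; Every Tick, it sets the widget's world rotation with FindLookAtRotation, aimed from the widget to that character's Camera.
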(event EventTick
  (params (DeltaSeconds :type Float%20%28single-precision%29))
  (Transformation|SetWorldRotation (Variables|Default|GetWidget) (Math|Rotator|FindLookatRotation (Transformation|GetWorldLocation (Variables|Default|GetWidget)) (Transformation|GetWorldLocation (Variables|/Game/a_TTD/GameMode/BP_TTD_Character.BP_TTD_Character_C|GetCamera (Variables|Default|GetAs%20BP%20TTD%20Character)))) false false))

(event EventBeginPlay
  (bind _asbp_ttd_character (Utilities|Casting|CastToBP_TTD_Character (Game|Player|GetPlayerPawn 0)))
  (Variables|Default|SetAs%20BP%20TTD%20Character _asbp_ttd_character))

(fn ConstructionScript)