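; BP_BombTower is a tower that, despite its name, attacks enemies with BP_Arrow projectiles.
; SetBuild extends the parent version and starts a looping cooldown timer that runs Find Nearest Enemy.
; That function sphere-traces down from ShootPoint, targets the first hit only if tagged Enemy rather than comparing distances, then plays a bow sound and fires a damage-carrying arrow from ShootPoint1.
; Upgrade is an empty stub.
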(event EventBeginPlay
  (|CallParentFunction))

(fn ConstructionScript
  (|CallParentFunction))

(fn FindNearestEnemy
  (bind _shootpoint (Variables|Default|GetShootPoint))
  (bind _returnvalue (Transformation|GetWorldLocation _shootpoint))
  (bind (_x _y _z) (Math|Vector|BreakVector _returnvalue))
  (bind (_outhit _returnvalue_2) (Collision|SphereTraceByChannel _returnvalue (Math|Vector|MakeVector _x _y (- _z 1e+04)) (Variables|Default|GetAttackRange) "TraceTypeQuery4" false 0 "None"))
  (if _returnvalue_2
    (if (Actor|ActorHasTag (.HitActor (Collision|BreakHitResult _outhit)) "Enemy")
      (bind _output_get (Variables|Default|SetTargetEnemy (.HitActor (Collision|BreakHitResult _outhit))))
      (Audio|PlaySoundatLocation "/Game/a_TTD/Audio/Cue_Attack_Bow.Cue_Attack_Bow" (Transformation|GetWorldLocation (Variables|Default|GetShootPoint1)) "0, 0, 0" 1.0 1.0 0.0 0 0 0)
      (bind _returnvalue_3 (Game|SpawnActorfromClass "/Game/a_TTD/Blueprints/BP_Arrow.BP_Arrow_C" (Math|Transform|MakeTransform (Transformation|GetWorldLocation (Variables|Default|GetShootPoint1)) (Math|Rotator|FindLookatRotation (Transformation|GetWorldLocation (Variables|Default|GetShootPoint1)) (Transformation|GetActorLocation _output_get)) "1,1,1") "Undefined" 0 0))
      (Default|SetDamageArrow _returnvalue_3 (Variables|Default|GetDamage))
      (Default|Shoot _returnvalue_3 (Variables|/Script/Engine.Actor|GetRootComponent (Variables|Default|GetTargetEnemy))))))

(fn SetBuild
  (|CallParentFunction)
  (Utilities|Time|SetTimerbyFunctionName 0 "Find Nearest Enemy" (Variables|Default|GetAttackCoolTime) true))

(fn Upgrade)