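; AI_Monster is an enemy in a tabletop tower defense game that attacks player towers and dies when its HP runs out.
; Overlapping a PlayerTower-tagged actor starts a looping Attack timer, which line-traces to that tower and damages the hit actor until the target is invalid.
; MoveToTower only picks the nearest tower from the game mode's list as TargetActor.
; Lethal damage swaps a material, then destroys the monster with an explosion.
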(event OnComponentBeginOverlap(Box)
  (params (OverlappedComponent :type Primitive%20Component%20Object%20Reference) (OtherActor :type Actor%20Object%20Reference) (OtherComp :type Primitive%20Component%20Object%20Reference) (OtherBodyIndex :type Integer) (bFromSweep :type Boolean) (SweepResult :type Hit%20Result%20Structure%20%28by%20ref%29))
  ;[1 1 1] 대상이 타워클래스라면
  (if (Actor|ActorHasTag OtherActor "PlayerTower")
    ;[1 1 1] 해당 엑터에 일정시간마다 공격 실행
    (Variables|Default|SetDamagedActor OtherActor)
    (Utilities|Time|SetTimerbyFunctionName 0 "Attack" 0.5 true)))

(event Game|Damage|EventAnyDamage
  (params (Damage :type Float%20%28single-precision%29) (DamageType :type Damage%20Type%20Object%20Reference) (InstigatedBy :type Controller%20Object%20Reference) (DamageCauser :type Actor%20Object%20Reference))
  (bind _output_get (Variables|Default|SetMonster%20HP (- (Variables|Default|GetMonster%20HP) Damage)))
  (if (<= _output_get 0.0)
    (Rendering|Material|SetMaterial (Variables|Default|Getstaticmesh) 1 "/Game/EF_FirstFloor/Common/Materials/SolidColor/OrangeMatte_Mat.OrangeMatte_Mat")
    (Utilities|FlowControl|Delay 0.1)
    (Actor|DestroyActor)
    (Effects|SpawnEmitteratLocation "/Game/StarterContent/Particles/P_Explosion.P_Explosion" (Transformation|GetActorLocation) "0, 0, 0" "3.000000,3.000000,3.000000")))

(fn ConstructionScript)

(fn Attack
  ;[1 1 1] 공격할 엑터가 유효한지 확인
  (Utilities|IsValid (Variables|Default|GetDamagedActor)
    (:Is%20Valid
      (bind (_outhit _returnvalue) (Collision|LineTraceByChannel (Transformation|GetActorLocation) (Transformation|GetActorLocation (Variables|Default|GetDamagedActor)) "TraceTypeQuery1" false 0 "None"))
      (if _returnvalue
        (Effects|SpawnEmitteratLocation "/Game/StarterContent/Particles/P_Explosion.P_Explosion" (+ (Transformation|GetActorLocation) (* (Math|Vector|GetForwardVector (Transformation|GetActorRotation)) 5e+01)) "0, 0, 0" "2.000000,2.000000,2.000000")
        (Game|Damage|ApplyDamage (.HitActor (Collision|BreakHitResult _outhit)) (Variables|Default|GetBase%20Damage) 0 0)))
    (:Is%20Not%20Valid
      (Utilities|Time|ClearTimerbyFunctionName 0 "Attack"))))

(fn MovetoTower
  (bind _asbp_gm_table_top_defense (Utilities|Casting|CastToBP_GM_TableTopDefense (Game|GetGameMode)))
  (Variables|Default|SettargetActor (.ReturnValue (Actor|FindNearestActor (Transformation|GetActorLocation) (Variables|/Game/a_TTD/GameMode/BP_GM_TableTopDefense.BP_GM_TableTopDefense_C|GetUpdateTowers _asbp_gm_table_top_defense)))))

(fn SetHP
  (params (Monster%20HP :type Float%20%28single-precision%29))
  (Variables|Default|SetMonster%20HP Monster%20HP))