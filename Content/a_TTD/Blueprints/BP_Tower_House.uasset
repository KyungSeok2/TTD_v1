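; House tower for the tabletop defense game that earns money for the player instead of showing any attack logic.
; Once built, a looping timer pays income into the game mode and briefly flashes a text amount that turns to face the player camera.
; Upgrade reads the game mode's upgrade level to swap mesh, income and health.
; AddDamage forwards zero damage to the parent; gold-actor spawning and timer clearing are unwired.
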(event EventTick
  (params (DeltaSeconds :type Float%20%28single-precision%29))
  (bind _textrender_money (Variables|Default|GetTextRender_Money))
  (bind _asbp_ttd_character (Utilities|Casting|CastToBP_TTD_Character (Game|Player|GetPlayerPawn 0)))
  (Transformation|SetWorldRotation _textrender_money (Math|Rotator|FindLookatRotation (Transformation|GetWorldLocation _textrender_money) (Transformation|GetWorldLocation (Variables|/Game/a_TTD/GameMode/BP_TTD_Character.BP_TTD_Character_C|GetCamera _asbp_ttd_character))) false false))

(fn ConstructionScript
  (|CallParentFunction))

(fn SetBuild
  (|CallParentFunction)
  (Utilities|Time|SetTimerbyFunctionName 0 "AddMoney" 5.0 true))

(fn AddMoney
  (Default|AddMoney (Variables|Default|GetTTD_GameMode) (Variables|Default|GetProduce%20Money))
  (Rendering|SetVisibility (Variables|Default|GetTextRender_Money) true false)
  (Utilities|Time|SetTimerbyFunctionName 0 "hidden Text" 0.7))

(fn Upgrade
  (switch Utilities|FlowControl|Switch|SwitchonBP_UpgradeLevel (Variables|/Game/a_TTD/GameMode/BP_GM_TableTopDefense.BP_GM_TableTopDefense_C|GetUpgrade%20Level%20 (Variables|Default|GetTTD_GameMode))
    (:NewEnumerator1
      (Components|StaticMesh|SetStaticMesh (Variables|Default|GetStaticMesh) "/Game/Low_Poly_Tower_Defense/Models/Props/SM_House_03.SM_House_03")
      (Variables|Default|SetProduce%20Money 10)
      (bind _output_get (Variables|Default|SetValue "+10"))
      (Rendering|Components|TextRender|SetText (Variables|Default|GetTextRender_Money) _output_get)
      (Variables|Default|SetMaxHP 2e+03)
      (Variables|Default|SetHP (+ (Variables|Default|GetHP) (Variables|Default|GetMaxHP))))
    (:NewEnumerator2
      (Components|StaticMesh|SetStaticMesh (Variables|Default|GetStaticMesh) "/Game/Low_Poly_Tower_Defense/Models/Props/SM_House_05.SM_House_05")
      (Variables|Default|SetProduce%20Money 20)
      (bind _output_get_2 (Variables|Default|SetValue "+20"))
      (Rendering|Components|TextRender|SetText (Variables|Default|GetTextRender_Money) _output_get_2)
      (Variables|Default|SetMaxHP 3e+03)
      (Variables|Default|SetHP (+ (Variables|Default|GetHP) (Variables|Default|GetMaxHP))))))

(fn HiddenText
  (Rendering|SetVisibility (Variables|Default|GetTextRender_Money) false false))

(fn AddDamage
  (params (Damage :type Float%20%28single-precision%29))
  (|CallParentFunction 0.0)
  (Actor|DestroyActor (Variables|Default|GetGoldActor)))