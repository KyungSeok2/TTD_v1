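; Game mode for the tabletop tower defense game, holding shared state for towers, money, upgrade level, castle and spawner count.
; Tower list changes and global upgrades go out through event dispatchers, with invalid towers pruned via a saved copy.
; Upgrades deduct money and report to the play widget, while added money is pushed to the castle.
; The last spawner's removal fades the camera and spawns the win widget actor; a lose counterpart also exists.
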(fn ConstructionScript)

(fn AddTower
  (params (UpdateTowers :type Actor%20Object%20Reference))
  (Utilities|Array|AddUnique (Variables|Default|GetUpdateTowers) UpdateTowers)
  (Variables|Default|SetSaveTowers (Variables|Default|GetUpdateTowers))
  ;[1 1 1] AI컨트롤러에 바인딩
  (Default|CallEventDispatcherUpdateTower))

(fn SetTowers
  (Utilities|Array|Clear (Variables|Default|GetUpdateTowers))
  (for _array_element (Variables|Default|GetSaveTowers)
    (Utilities|IsValid _array_element
      (:Is%20Valid
        (Utilities|Array|AddUnique (Variables|Default|GetUpdateTowers) _array_element))))
  (Variables|Default|SetSaveTowers (Variables|Default|GetUpdateTowers))
  ;[1 1 1] AI컨트롤러에 바인딩
  (Default|CallEventDispatcherUpdateTower))

(fn AddMoney
  (params (Add%20Money :type Integer))
  (bind _bp_t_castle (Variables|Default|GetBP%20T%20Castle))
  (bind _output_get (Variables|Default|SetMoney (+ (Variables|Default|GetMoney) Add%20Money)))
  (Utilities|IsValid _bp_t_castle
    (:Is%20Valid
      (Default|SetMoney _bp_t_castle _output_get))
    (:Is%20Not%20Valid
      (Development|PrintString "zzzzzzzzzzzzzzzzzz" true true "(R=0.000000,G=0.660000,B=1.000000,A=1.000000)" 6e+01))))

(fn UseMoney
  (params (UseMoney :type Integer))
  (Variables|Default|SetMoney (- (Variables|Default|GetMoney) UseMoney)))

(fn Upgrade
  (if (Utilities|Enum|NotEqual(Enum) (Variables|Default|GetUpgrade%20Level%20) "NewEnumerator2")
    (CallFunction|UseMoney 3000)
    (switch Utilities|FlowControl|Switch|SwitchonBP_UpgradeLevel (Variables|Default|GetUpgrade%20Level%20)
      (:NewEnumerator0
        (Default|UpgradeComlete (Variables|Default|GetBP%20Widget%20Play))
        (Variables|Default|SetUpgrade%20Level%20 "NewEnumerator1")
        ;[1 1 1] 타워에 바인딩
        (Default|CallEventDispatcherUpgrade :!label _label))
      (:NewEnumerator1
        (Default|UpgradeComlete (Variables|Default|GetBP%20Widget%20Play))
        (Variables|Default|SetUpgrade%20Level%20 "NewEnumerator2")
        (goto _label))
      (:NewEnumerator2
        (Default|CantUpgrade (Variables|Default|GetBP%20Widget%20Play))))))

(fn GetWidget
  (bind _asbp_ttd_character (Utilities|Casting|CastToBP_TTD_Character (Game|Player|GetPlayerPawn 0)))
  (bind _asbp_widget_play (Utilities|Casting|CastToBP_Widget_Play (UserInterface|GetWidget (Variables|/Game/a_TTD/Blueprints/BP_WidgetActor_Play.BP_WidgetActor_Play_C|GetWidget (Variables|/Game/a_TTD/GameMode/BP_TTD_Character.BP_TTD_Character_C|GetPlayWidgetActor _asbp_ttd_character)))))
  (Variables|Default|SetBP%20Widget%20Play _asbp_widget_play))

(fn AddSpawner
  (Variables|Default|SetSpawner%20Num (+ (Variables|Default|GetSpawner%20Num) 1)))

(fn DeleteSpawner
  (bind _output_get (Variables|Default|SetSpawner%20Num (- (Variables|Default|GetSpawner%20Num) 1)))
  (if (<= _output_get 0)
    (CameraFades|StartCameraFade :self (Game|GetPlayerCameraManager 0) :ToAlpha 1.0 :Duration 1.0)
    (CallFunction|WinWidget)))

(fn AddCastle
  (params (Castle :type Actor%20Object%20Reference))
  (bind _asbp_t_castle_ (Utilities|Casting|CastToBP_T_Castle_ Castle))
  (Variables|Default|SetBP%20T%20Castle _asbp_t_castle_))

(fn LoseWidget
  (Game|SpawnActorfromClass "/Game/a_TTD/Blueprints/BP_WidgetActor_Lose.BP_WidgetActor_Lose_C" (Math|Transform|MakeTransform "0, 0, 0" "0,165.000000, 0" "20.000000,20.000000,20.000000") "Undefined" 0 0))

(fn WinWidget
  (Game|SpawnActorfromClass "/Game/a_TTD/Blueprints/BP_WidgetActor_Win.BP_WidgetActor_Win_C" (Math|Transform|MakeTransform "0, 0, 0" "0,165.000000, 0" "20.000000,20.000000,20.000000") "Undefined" 0 0))